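; BP_Door is a door that opens when a BP_ThirdPersonCharacter overlaps its DoorTrigger.
; The first overlap caches the starting relative Y of the Sphere component, which acts as the moving door part.
; The DoorOpen timeline then slides that component along Y from the cached position and changes its pitch, using separate move and open tracks.
; No logic closes it.
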(event `self.DoorTrigger.OnComponentBeginOverlap`
  (params (OverlappedComponent :type "PrimitiveComponent Object Reference") (OtherActor :type "Actor Object Reference") (OtherComp :type "PrimitiveComponent Object Reference") (OtherBodyIndex :type Integer) (bFromSweep :type Boolean) (SweepResult :type "HitResult Structure (by ref)"))
  (bind _sphere (`self.Sphere`))
  (bind (_relativelocation_x _relativelocation_y _relativelocation_z) (`KismetMathLibrary.BreakVector` (`SceneComponent.RelativeLocation` _sphere)))
  (bind (_relativelocation_x_2 _relativelocation_y_2) (`KismetMathLibrary.BreakVector` (`SceneComponent.RelativeLocation` (`self.Sphere`))))
  (cast `/Game/ThirdPerson/Blueprints/BP_ThirdPersonCharacter` OtherActor)
  (if (`self.IsPosSet`)
    (bind (_direction _dooropen _doormove) (`Timeline|DoorOpen` :!label _label)
      (:`Update`
        (`SceneComponent.K2_SetRelativeLocationAndRotation` _sphere (`KismetMathLibrary.MakeVector` _relativelocation_x (+ (* _doormove 200.0) (`self.Original_pos`)) _relativelocation_z) (`KismetMathLibrary.MakeRotator` 0.0 (* _dooropen 90.0) -90.0) false false)))
    (else
      (set `self.IsPosSet` true)
      (set `self.Original_pos` _relativelocation_y_2)
      (goto _label))))

(fn `UserConstructionScript`)